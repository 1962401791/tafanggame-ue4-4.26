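; Tower-defense turret base (taji) that starts at level 0, upgrades through five levels with new meshes, and can be sold back to empty.
; A level-scaled sphere trace, polled by timer while idle, picks a random enemy.
; Tick aims the mesh, retargets on death or beyond a fixed range, and spawns bullets with level-based damage, material and delay-gated fire rate.
; Clicking it opens the Levelup widget at the cursor.
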(event Custom|levelup
  (bind _等级 (Variables|Default|Get等级))
  (if (<= _等级 4)
    (Math|Integer|IncrementInt _等级
      (:%20%20
        (Rendering|SetVisibility (Variables|Default|GetSkeletalMesh) true false)
        (Class|SkinnedMeshComponent|SetSkeletalMesh (Variables|Default|GetSkeletalMesh) (Utilities|Select :Index (Variables|Default|Get等级) :Option%200 0 :Option%201 "/Game/CSC/Meshes/SK_CSC_Gun4.SK_CSC_Gun4" :Option%202 "/Game/CSC/Meshes/SK_CSC_Base1.SK_CSC_Base1" :Option%203 "/Game/CSC/Meshes/SK_TANK_Base1.SK_TANK_Base1" :Option%204 "/Game/CSC/Meshes/SK_RLV_Base1.SK_RLV_Base1" :Option%205 "/Game/CSC/Meshes/SK_LGT_Base1.SK_LGT_Base1") true)))))

(event Custom|重新检查敌人
  (bind _self self)
  (bind _allenemy (Variables|Default|GetallEnemy))
  (bind _returnvalue (Transformation|GetActorLocation _self))
  ;[1 1 1] 检测敌人
  (if (> (Variables|Default|Get等级) 0)
    (Utilities|Array|Clear (Variables|Default|GetallEnemy))
    (bind _outhits (Collision|MultiSphereTraceForObjects _returnvalue _returnvalue (Utilities|Select :Index (Variables|Default|Get等级) :Option%200 0.0 :Option%201 5e+02 :Option%202 6e+02 :Option%203 7e+02 :Option%204 8e+02 :Option%205 9e+02) (Utilities|Array|MakeArray "ObjectTypeQuery3") false 0 "None"))
    (for _array_element _outhits
      (bind _asenemy (Utilities|Casting|CastToenemy (.HitActor (Collision|BreakHitResult _array_element))))
      (Utilities|Array|Add (Variables|Default|GetallEnemy) _asenemy))
    (if (== (Utilities|Array|Length (Variables|Default|GetallEnemy)) 0)
      (bind _returnvalue_2 (Utilities|Time|SetTimerbyEvent (delegate Custom|检测周围有没有敌人) 0.5 true))
      (Variables|Default|Setselectenemy _returnvalue_2)
      (else
        (Variables|Default|Setnowenemy (Utilities|Array|Get(acopy) _allenemy (Math|Random|RandomIntegerinRange 0 (- (Utilities|Array|Length _allenemy) 1))))
        (Utilities|Time|ClearandInvalidateTimerbyHandle (Variables|Default|Getselectenemy))))))

(event Custom|发射子弹
  (if (Variables|Default|Getshotbullet?)
    (bind _nowenemy (Variables|Default|Getnowenemy)
      (:then
        (Game|SpawnActorfromClass "/Game/blueprint/bullet/1bullet_Child.1bullet_Child_C" (Transformation|GetActorTransform) "Undefined" 0 _nowenemy (* 15 (Math|Conversions|ToFloat(Integer) (Variables|Default|Get等级))) (Utilities|Select :Index (Variables|Default|Get等级) :Option%200 0 :Option%201 "/Game/CSC/Demo/Materials/M_Bullet.M_Bullet" :Option%202 "/Game/CSC/Demo/Materials/M_Bullet1.M_Bullet1" :Option%203 "/Game/CSC/Demo/Materials/M_Bullet1_2.M_Bullet1_2" :Option%204 "/Game/CSC/Demo/Materials/M_Bullet1_3.M_Bullet1_3" :Option%205 "/Game/CSC/Demo/Materials/M_Bullet1_4.M_Bullet1_4") 0)
        (Variables|Default|Setshotbullet? false))
      (:else))
    (else
      (Utilities|FlowControl|Delay (Utilities|Select :Index (Variables|Default|Get等级) :Option%200 1.0 :Option%201 1.2 :Option%202 1.1 :Option%203 0.9 :Option%204 0.6 :Option%205 0.3))
      (Variables|Default|Setshotbullet? true))))

(event Custom|sell
  (Variables|Default|Set等级 0)
  (Rendering|SetVisibility (Variables|Default|GetSkeletalMesh) false false))

(event Custom|检测周围有没有敌人
  (bind _self self)
  (bind _allenemy (Variables|Default|GetallEnemy))
  (bind _returnvalue (Transformation|GetActorLocation _self))
  ;[1 1 1] 检测敌人
  (Utilities|Array|Clear (Variables|Default|GetallEnemy))
  (bind _outhits (Collision|MultiSphereTraceForObjects _returnvalue _returnvalue (Utilities|Select :Index (Variables|Default|Get等级) :Option%200 0.0 :Option%201 5e+02 :Option%202 6e+02 :Option%203 7e+02 :Option%204 8e+02 :Option%205 9e+02) (Utilities|Array|MakeArray "ObjectTypeQuery3") false 0 "None"))
  (for _array_element _outhits
    (bind _asenemy (Utilities|Casting|CastToenemy (.HitActor (Collision|BreakHitResult _array_element))))
    (Utilities|Array|Add (Variables|Default|GetallEnemy) _asenemy))
  (if (not (== (Utilities|Array|Length (Variables|Default|GetallEnemy)) 0))
    (Variables|Default|Setnowenemy (Utilities|Array|Get(acopy) _allenemy (Math|Random|RandomIntegerinRange 0 (- (Utilities|Array|Length _allenemy) 1))))
    (Utilities|Time|ClearandInvalidateTimerbyHandle (Variables|Default|Getselectenemy))))

(event EventBeginPlay
  ;[1 1 1] 检测敌人
  (bind _returnvalue (Utilities|Time|SetTimerbyEvent (delegate Custom|检测周围有没有敌人) 0.5 true))
  (Variables|Default|Setselectenemy _returnvalue))

(event Collision|EventActorBeginOverlap
  (params (OtherActor :type Actor%20Object%20Reference)))

(event MouseInput|EventActorOnClicked
  (params (ButtonPressed :type Key%20Structure))
  ;[1 1 1] 点击taji显示ui
  (bind _foundwidgets (Widget|GetAllWidgetsOfClass "/Game/UI/levelup.levelup_C" true))
  (for _array_element _foundwidgets
    (Widget|RemovefromParent _array_element))
  (bind _returnvalue (UserInterface|CreateWidget "/Game/UI/levelup.levelup_C" 0 (Variables|Default|Get等级) self))
  (UserInterface|Viewport|AddtoViewport _returnvalue 0)
  (bind _returnvalue_2 (Class|WidgetLayoutLibrary|GetMousePositiononViewport))
  (Class|UserWidget|SetPositioninViewport _returnvalue _returnvalue_2 false))

(event EventTick
  (params (DeltaSeconds :type Float%20%28single-precision%29))
  (if (> (Variables|Default|Get等级) 0)
    (Utilities|IsValid (Variables|Default|Getnowenemy)
      (:Is%20Valid
        (if (Variables|/Game/blueprint/enemy/enemy.enemy_C|Getdie (Variables|Default|Getnowenemy))
          (CallFunction|重新检查敌人 :!label _label)
          (else
            (Transformation|SetWorldRotation (Variables|Default|GetSkeletalMesh) (Math|Rotator|FindLookatRotation (Transformation|GetWorldLocation (Variables|Default|GetSkeletalMesh)) (Transformation|GetActorLocation (Variables|Default|Getnowenemy))) false false)
            (if (>= (Math|Vector|VectorLength (- (Transformation|GetWorldLocation (Variables|Default|GetSkeletalMesh)) (Transformation|GetActorLocation (Variables|Default|Getnowenemy)))) 9e+02)
              (Variables|Default|Setnowenemy 0)
              (CallFunction|重新检查敌人)
              (else
                (CallFunction|发射子弹))))))
      (:Is%20Not%20Valid
        (goto _label)))))

(fn ConstructionScript)