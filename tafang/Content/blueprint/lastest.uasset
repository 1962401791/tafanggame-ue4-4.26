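; Trigger actor that acts as a damage point for enemies, draining the HP stored in the game mode.
; When an enemy overlaps its Box component, that enemy's Damage is subtracted from HP on 1gamemode and the enemy is destroyed.
; If HP drops to zero or below, it only prints a death message; no other game-over logic runs here.
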(event OnComponentBeginOverlap(Box)
  (params (OverlappedComponent :type Primitive%20Component%20Object%20Reference) (OtherActor :type Actor%20Object%20Reference) (OtherComp :type Primitive%20Component%20Object%20Reference) (OtherBodyIndex :type Integer) (bFromSweep :type Boolean) (SweepResult :type Hit%20Result%20Structure%20%28by%20ref%29))
  (bind _returnvalue (Game|GetGameMode))
  (bind _as1gamemode (Utilities|Casting|CastTo1gamemode _returnvalue))
  (bind _asenemy (Utilities|Casting|CastToenemy OtherActor))
  (bind _output_get (Variables|/Game/1game/1gamemode.1gamemode_C|SetHP _as1gamemode (- (Variables|/Game/1game/1gamemode.1gamemode_C|GetHP _as1gamemode) (Variables|/Game/blueprint/enemy/enemy.enemy_C|Getdamage _asenemy))))
  (Actor|DestroyActor _asenemy)
  (if (<= _output_get 0.0)
    (Development|PrintText "you die")))

(event EventBeginPlay)

(event Collision|EventActorBeginOverlap
  (params (OtherActor :type Actor%20Object%20Reference)))

(event EventTick
  (params (DeltaSeconds :type Float%20%28single-precision%29)))

(fn ConstructionScript)