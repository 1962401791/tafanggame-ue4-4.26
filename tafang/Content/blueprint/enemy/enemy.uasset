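; Enemy actor Blueprint for what appears to be a path-based defense game with several skeleton enemy types.
; After a short delay it walks a linked chain of road actors from its Start's first road, using repeated AIMoveTo calls.
; Damage lowers HP; on death a DoOnce randomly picks an ID-selected death animation or ragdoll, destroys the actor and adds Value to game mode Money.
; Death of ID 1 also calls WingameMessage.
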(event EventBeginPlay
  ;[1 1 1] 敌人移动
  (Utilities|FlowControl|Delay 0.5)
  (if (Variables|Default|Getstartisvalid?)
    (Variables|Default|Setnextroad (Variables|/Game/blueprint/start.start_C|Getfirstroad (Variables|Default|Getstart)))
    (AI|AIMoveTo self "0, 0, 0" (Variables|Default|Getnextroad) 5.0 false :!label _label
      (:OnSuccess
        (bind _output_get (Variables|Default|Setnextroad (Variables|/Game/blueprint/end.end_C|Getroad (Variables|Default|Getnextroad))))
        (Utilities|IsValid _output_get
          (:Is%20Valid
            (goto _label)))))))

(event Collision|EventActorBeginOverlap
  (params (OtherActor :type Actor%20Object%20Reference)))

(event EventTick
  (params (DeltaSeconds :type Float%20%28single-precision%29)))

(event Game|Damage|EventAnyDamage
  (params (Damage :type Float%20%28single-precision%29) (DamageType :type Damage%20Type%20Object%20Reference) (InstigatedBy :type Controller%20Object%20Reference) (DamageCauser :type Actor%20Object%20Reference))
  (bind _returnvalue (Game|GetGameMode))
  (bind _as1gamemode (Utilities|Casting|CastTo1gamemode _returnvalue))
  ;[1 1 1] 敌人是否死亡，以及死亡后的动画播放
  (bind _output_get (Variables|Default|SetHP (- (Variables|Default|GetHP) Damage)))
  (if (<= _output_get 0.0)
    (Variables|Default|Setdie true)
    (if (== (Variables|Default|GetID) 1)
      (Class|Gamebpi|Wingame(Message) self))
    (Utilities|FlowControl|DoOnce false
      (:Completed
        (Utilities|FlowControl|MultiGate true false -1
          (:Out%200
            (Components|Animation|PlayAnimation (Variables|Character|GetMesh) (Utilities|Select :Index (Variables|Default|GetID) :Option%200 0 :Option%201 "/Game/SkeletonCrew/Skeleton_Crossbowman/Animations/Skeleton_Crossbowman_Die.Skeleton_Crossbowman_Die" :Option%202 "/Game/SkeletonCrew/Skeleton_Grunt/Animations/Skeleton_Grunt_Death.Skeleton_Grunt_Death" :Option%203 "/Game/SkeletonCrew/Skeleton_King/Animations/Skeleton_King_Death.Skeleton_King_Death" :Option%204 "/Game/SkeletonCrew/Skeleton_Mage/Animations/Skeleton_Mage_Die.Skeleton_Mage_Die" :Option%205 "/Game/SkeletonCrew/Skeleton_Swordman/Animations/Skeleton_Swordman_Die.Skeleton_Swordman_Die") false)
            (Utilities|FlowControl|Delay 0.3)
            (Actor|DestroyActor))
          (:Out%201
            (Physics|SetSimulatePhysics (Variables|Character|GetMesh) true)
            (Utilities|FlowControl|Delay 0.3)
            (Actor|DestroyActor)))
        (Variables|/Game/1game/1gamemode.1gamemode_C|Setmoney _as1gamemode (+ (Variables|/Game/1game/1gamemode.1gamemode_C|Getmoney _as1gamemode) (Variables|Default|Getvalue)))))))

(fn ConstructionScript)