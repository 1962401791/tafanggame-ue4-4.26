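; Enemy Blueprint variant, child of a parent enemy class, whose death ends the game as a win.
; Tick watches the Die flag and, once it is set on a valid actor, uses a DoOnce to fire a single win call.
; The win event casts the current game mode to 1gamemode and calls Gamewin.
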(event Custom|win
  (bind _as1gamemode (Utilities|Casting|CastTo1gamemode (Game|GetGameMode)))
  (Default|Gamewin _as1gamemode))

(event EventBeginPlay)

(event Collision|EventActorBeginOverlap
  (params (OtherActor :type Actor%20Object%20Reference)))

(event EventTick
  (params (DeltaSeconds :type Float%20%28single-precision%29))
  (if (Variables|Default|Getdie)
    (Utilities|IsValid self
      (:Is%20Valid
        (Utilities|FlowControl|DoOnce false
          (:Completed
            (CallFunction|Win)))))))

(fn ConstructionScript
  (|CallParentFunction))