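; Homing bullet actor that chases a selected enemy and damages it on contact.
; Each tick it steers toward the target via look-at rotation, setting local-space velocity at a speed picked from a table indexed by damage divided by ten.
; Overlapping an enemy with its box applies the damage and destroys the bullet; losing a valid target destroys it after a short delay.
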(event OnComponentBeginOverlap(Box)
  (params (OverlappedComponent :type Primitive%20Component%20Object%20Reference) (OtherActor :type Actor%20Object%20Reference) (OtherComp :type Primitive%20Component%20Object%20Reference) (OtherBodyIndex :type Integer) (bFromSweep :type Boolean) (SweepResult :type Hit%20Result%20Structure%20%28by%20ref%29))
  ;[1 1 1] 子弹造成伤害后销毁
  (bind _asenemy (Utilities|Casting|CastToenemy OtherActor))
  (Game|Damage|ApplyDamage _asenemy (Variables|Default|Getdamage1) 0 0)
  (Actor|DestroyActor))

(event EventBeginPlay
  (Rendering|Material|SetMaterial (Variables|Default|GetSphere) 0 (Variables|Default|GetMaterial)))

(event EventTick
  (params (DeltaSeconds :type Float%20%28single-precision%29))
  ;[1 1 1] 子弹跟追敌人直至死亡
  (bind _selectedenemy (Variables|Default|Getselectedenemy)
    (:then
      (Game|Components|ProjectileMovement|SetVelocityinLocalSpace (Variables|Default|GetProjectileMovement) (* (Math|Rotator|GetRotationXVector (Math|Rotator|FindLookatRotation (Transformation|GetActorLocation) (Transformation|GetActorLocation _selectedenemy))) (Utilities|Select :Index (Math|Float|Truncate (/ (Variables|Default|Getdamage1) 1e+01)) :Option%200 0.0 :Option%201 1.5e+03 :Option%202 1.8e+03 :Option%203 2.25e+03 :Option%204 2e+03 :Option%205 2.5e+03))))
    (:else
      (Utilities|FlowControl|Delay 0.2)
      (Actor|DestroyActor))))

(fn ConstructionScript)